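; Demo player controller that boots the BDCUI demo interface on BeginPlay.
; It retries each tick until a valid HUD exists, then casts and caches it as HUD_BDCUI_Demo.
; Through that HUD it spawns the widget viewport, shows the cursor and adds the main demo widget to the prompt container.
; It then spawns and stores a BP_RecordingActor high above the world origin, flagged as player view.
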(event `self.ReceiveBeginPlay`
  (`/Engine/EditorBlueprintResources/StandardMacros.IsValid` (`self.GetHUD`) :!label _label ; Only proceed, if a AHUD is spawned.\nElse, Rebegin this
    (:`Is Valid`
      (`self.Self_HUD` ; Check if a HUD is stored.
        (:`then`
          _)
        (:`else`
          (bind _ashud_bdcui_demo (cast `/BDC_UI_Library/Demonstration/HUD_BDCUI_Demo` (`self.GetHUD`))) ; Take the spawned HUD and cast it to the\nowning one. If passed, store it.
          (set `self.Self_HUD` _ashud_bdcui_demo)))
      (`/BDC_UI_Library/Demonstration/HUD_BDCUI_Demo.SpawnViewport` (`self.Self_HUD`) self) ; Spawn the actual Viewport to drop\nWidgets inside
      (set `self.bShowMouseCursor` true) ; enable Cursor
      (`/BDC_UI_Library/Demonstration/HUD_BDCUI_Demo.HUD_AddWidget` :`self` (`self.Self_HUD`) :`CreatingWidget` "/BDC_UI_Library/Demonstration/Widgets_Demo/BDCUI_Demo_Main.BDCUI_Demo_Main_C" :`IntoContainer` "ContainerPrompt") ; Add a Widget to the HUD.\nThe corresponding Function is implemented in the\nSelf_HUD
      (bind _returnvalue (`|SpawnActorFromClass` "/BDC_UI_Library/CommonBases/BP_RecordingActor.BP_RecordingActor_C" (`KismetMathLibrary.MakeTransform` (0.0 0.0 10000.0)) "AlwaysSpawn" "MultiplyWithRoot" null 240.0 true 0 null))
      (set `self.Actor_Recording` _returnvalue))
    (:`Is Not Valid`
      (`self.ReBegin`))))

(event `ReBegin`
  (`KismetSystemLibrary.DelayUntilNextTick`)
  (goto _label))

(fn `UserConstructionScript`)