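; BDC_UI_Demo_BP is a demonstration Blueprint that lays out sample nodes from the BDC UI plugin, with no gameplay behavior of its own.
; Its event graph shows BDCUISubsystem calls for widget selection, current UI and last-of-UI tracking.
; It also shows function library helpers for panel slots, Enhanced Input and CommonUI key lookups, key icons and widget geometry.
; No node is wired to an event, and the construction script is empty.
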(fn `UserConstructionScript`)