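; Preview-capture actor that renders only itself, with a swappable skeletal mesh, into a render target for the player view or one of four NPC slots.
; The construction script picks the target from IsPlayerView and NPCID; ClipActor triggers each capture manually.
; CameraArm yaw turns by velocity or through looping-timer lerps to an angle or initial yaw, guarded by DoOnce.
; ChangeMesh swaps the mesh, optionally resetting yaw, or hides it when invalid.
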(event `self.ReceiveBeginPlay`
  (set `SceneCaptureComponent.ShowOnlyActors` (`|MakeArray` self :!type "Actor Object Reference") (`self.SceneCaptureComponent2D`)))

(event `RotateByVelocity`
  (params (velocity :type "Float (double-precision)"))
  (`SceneComponent.K2_AddRelativeRotation` (`self.CameraArm`) (`KismetMathLibrary.MakeRotator` 0.0 0.0 velocity) false false))

(event `RotateByAngle`
  (params (Angle :type "Float (double-precision)") (Duration :type "Float (double-precision)"))
  (bind (_relativerotation_roll _relativerotation_pitch _relativerotation_yaw) (`KismetMathLibrary.BreakRotator` (`SceneComponent.RelativeRotation` (`self.CameraArm`))))
  (if (not (`KismetSystemLibrary.K2_IsValidTimerHandle` (`self.LerpHandle`)))
    (`/Engine/EditorBlueprintResources/StandardMacros.DoOnce` false :!label _label
      (:`Completed`
        (set `self.BeforeYaw` _relativerotation_yaw)
        (set `self.DurationStep` (/ 1.0 (* Duration 10.0)))
        (set `self.TargetYaw` (+ (`self.BeforeYaw`) Angle))
        (set `self.CurrentAlpha` 0.0)
        (bind _returnvalue (`KismetSystemLibrary.K2_SetTimerDelegate` (delegate `Lerping`) 0.01 true))
        (set `self.LerpHandle` _returnvalue)))))

(event `ResetRotator`
  (goto _label :!via `Reset`))

(event `Lerping`
  (`SceneComponent.K2_SetRelativeRotation` (`self.CameraArm`) (`KismetMathLibrary.MakeRotator` 0.0 0.0 (`KismetMathLibrary.Lerp` (`self.BeforeYaw`) (`self.TargetYaw`) (`self.CurrentAlpha`))) false false)
  (set `self.CurrentAlpha` (+ (`self.CurrentAlpha`) (`self.DurationStep`)))
  (if (> (`self.CurrentAlpha`) 1.0)
    (`KismetSystemLibrary.K2_ClearAndInvalidateTimerHandle` (`self.LerpHandle`))
    (`SceneComponent.K2_SetRelativeRotation` (`self.CameraArm`) (`KismetMathLibrary.MakeRotator` 0.0 0.0 (`self.TargetYaw`)) false false)
    (`self.ResetRotator`)))

(event `ClipActor`
  (`SceneCaptureComponent2D.CaptureScene` (`self.SceneCaptureComponent2D`)))

(event `RotateReset`
  (params (Duration :type "Float (double-precision)"))
  (bind (_relativerotation_roll _relativerotation_pitch _relativerotation_yaw) (`KismetMathLibrary.BreakRotator` (`SceneComponent.RelativeRotation` (`self.CameraArm`))))
  (if (not (`KismetSystemLibrary.K2_IsValidTimerHandle` (`self.LerpHandle`)))
    (`/Engine/EditorBlueprintResources/StandardMacros.DoOnce` false :!label _label_2
      (:`Completed`
        (set `self.BeforeYaw` _relativerotation_yaw)
        (set `self.DurationStep` (/ 1.0 (* Duration 10.0)))
        (set `self.TargetYaw` (`self.InitializeYaw`))
        (set `self.CurrentAlpha` 0.0)
        (bind _returnvalue (`KismetSystemLibrary.K2_SetTimerDelegate` (delegate `LerpReset`) 0.01 true))
        (set `self.LerpHandle` _returnvalue)))))

(event `ResetReset`
  (goto _label_2 :!via `Reset`))

(event `LerpReset`
  (`SceneComponent.K2_SetRelativeRotation` (`self.CameraArm`) (`KismetMathLibrary.MakeRotator` 0.0 0.0 (`KismetMathLibrary.Lerp` (`self.BeforeYaw`) (`self.TargetYaw`) (`self.CurrentAlpha`))) false false)
  (set `self.CurrentAlpha` (+ (`self.CurrentAlpha`) (`self.DurationStep`)))
  (if (> (`self.CurrentAlpha`) 1.0)
    (`KismetSystemLibrary.K2_ClearAndInvalidateTimerHandle` (`self.LerpHandle`))
    (`SceneComponent.K2_SetRelativeRotation` (`self.CameraArm`) (`KismetMathLibrary.MakeRotator` 0.0 0.0 (`self.InitializeYaw`)) false false)
    (`self.ResetReset`)))

(event `ChangeMesh`
  (params (NewMesh :type "SkeletalMesh Object Reference") (ResetRotation :type Boolean) (NewInitRotation :type "Float (double-precision)") (OfNPC :type Integer))
  (`/Engine/EditorBlueprintResources/StandardMacros.IsValid` NewMesh
    (:`Is Valid`
      (`SkeletalMeshComponent.SetSkeletalMeshAsset` (`self.SkeletalMesh`) NewMesh)
      (if ResetRotation
        (set `self.InitializeYaw` NewInitRotation)
        (`self.RotateReset` 0.0)
        (`SceneComponent.SetVisibility` (`self.SkeletalMesh`) true false)
        (set `self.NPC_ID` OfNPC)))
    (:`Is Not Valid`
      (`SceneComponent.SetVisibility` (`self.SkeletalMesh`) false false)
      (`KismetSystemLibrary.PrintString` "not valid"))))

(fn `UserConstructionScript`
  (set `SceneCaptureComponent.ShowOnlyActors` (`|MakeArray` self :!type "Actor Object Reference") (`self.SceneCaptureComponent2D`))
  (`SceneComponent.K2_SetRelativeRotation` (`self.CameraArm`) (`KismetMathLibrary.MakeRotator` 0.0 0.0 (`self.InitializeYaw`)) false false)
  (set `self.NPC_ID` (`KismetMathLibrary.Clamp` (`self.NPC_ID`) 0 3))
  (if (`self.isPlayerView`)
    (set `SceneCaptureComponent2D.TextureTarget` "/BDC_UI_Library/CommonMaterials/Tex_Captures/Capture_ActorRenderTarget_Player.Capture_ActorRenderTarget_Player" (`self.SceneCaptureComponent2D`))
    (else
      (set `SceneCaptureComponent2D.TextureTarget` (select `int` (`self.NPC_ID`) :`0` "/BDC_UI_Library/CommonMaterials/Tex_Captures/Capture_ActorRenderTarget_NPC_0.Capture_ActorRenderTarget_NPC_0" :`1` "/BDC_UI_Library/CommonMaterials/Tex_Captures/Capture_ActorRenderTarget_NPC_1.Capture_ActorRenderTarget_NPC_1" :`2` "/BDC_UI_Library/CommonMaterials/Tex_Captures/Capture_ActorRenderTarget_NPC_2.Capture_ActorRenderTarget_NPC_2" :`3` "/BDC_UI_Library/CommonMaterials/Tex_Captures/Capture_ActorRenderTarget_NPC_3.Capture_ActorRenderTarget_NPC_3" :!type "TextureRenderTarget2D Object Reference") (`self.SceneCaptureComponent2D`)))))